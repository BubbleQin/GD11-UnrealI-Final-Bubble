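; BP_LevelTarget is a level objective actor that counts target kills, then signals completion and destroys itself once the goal is reached.
; GetSpawnTranses builds enemy spawn transforms from random reachable navmesh points within a radius of the actor.
; CheckSpawnTrans only iterates those transforms with an empty loop body; its debug sphere drawing is disconnected.
; OnSpawnEnemies is empty here, so this Blueprint does no spawning itself.
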(event Custom|CheckSpawnTrans
  (bind _outtrans (CallFunction|GetSpawnTranses))
  (for _array_element _outtrans
    _))

(event EventBeginPlay)

(event Collision|EventActorBeginOverlap
  (params (OtherActor :type Actor%20Object%20Reference)))

(event EventTick
  (params (DeltaSeconds :type Float%20%28single-precision%29)))

(fn ConstructionScript)

(fn OnTargetKilled
  (bind _output_get (Variables|Default|SetTargetKilledNum (+ (Variables|Default|GetTargetKilledNum) 1)))
  (if (>= _output_get (Variables|Default|GetTargetKilledGoal))
    (Utilities|FlowControl|DoOnce false
      (:Completed
        (Default|CallTargetFinished)
        (Actor|DestroyActor)))))

(fn OnSpawnEnemies)

(fn GetSpawnTranses
  (bind _trans (LocalVariables|GetTrans))
  (for _index (range 0 (- (Variables|Default|GetEnemyNum) 1))
    (Utilities|Array|Add _trans (Math|Transform|MakeTransform (.RandomLocation (AI|Navigation|GetRandomReachablePointinRadius (Transformation|GetActorLocation) (Variables|Default|GetRadius) 0 0)))))
  (return _trans))